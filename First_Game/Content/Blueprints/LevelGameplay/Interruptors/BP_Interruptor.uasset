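; BP_Interruptor is a floor switch that reacts while the player character stands on it.
; Box overlap events filter for BP_PlayerCharacter, pressing the button on entry and releasing it on exit.
; Pressing flattens and lowers the Button component instantly, with no animation, and releasing restores its height.
; Each state change calls OnInterruptorActivated or OnInterruptorDesactivated, presumably event dispatchers for other actors to react to.
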(event `ActivateButton`
  (`SceneComponent.SetRelativeScale3D` (`self.Button`) (0.3 0.3 0.05))
  (`SceneComponent.K2_SetRelativeLocation` (`self.Button`) (0.0 0.0 5.0) false false)
  (`self.OnInterruptorActivated`))

(event `DesactivateButton`
  (`SceneComponent.SetRelativeScale3D` (`self.Button`) (0.3 0.3 0.3))
  (`SceneComponent.K2_SetRelativeLocation` (`self.Button`) (0.0 0.0 15.0) false false)
  (`self.OnInterruptorDesactivated`))

(event `self.Box.OnComponentBeginOverlap`
  (params (OverlappedComponent :type "PrimitiveComponent Object Reference") (OtherActor :type "Actor Object Reference") (OtherComp :type "PrimitiveComponent Object Reference") (OtherBodyIndex :type Integer) (bFromSweep :type Boolean) (SweepResult :type "HitResult Structure (by ref)"))
  (cast `/Game/Blueprints/PlayerCharacter/BP_PlayerCharacter` OtherActor)
  (`self.ActivateButton`))

(event `self.Box.OnComponentEndOverlap`
  (params (OverlappedComponent :type "PrimitiveComponent Object Reference") (OtherActor :type "Actor Object Reference") (OtherComp :type "PrimitiveComponent Object Reference") (OtherBodyIndex :type Integer))
  (cast `/Game/Blueprints/PlayerCharacter/BP_PlayerCharacter` OtherActor)
  (`self.DesactivateButton`))

(fn `UserConstructionScript`)