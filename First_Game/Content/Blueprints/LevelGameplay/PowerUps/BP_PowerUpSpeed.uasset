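; Speed power-up pickup that temporarily raises a player character's max walk speed.
; Overlapping its box with a BP_PlayerCharacter stores that character, hides the pickup, disables its collision and adds SpeedBuff to MaxWalkSpeed.
; After a Delay of Duration, the pickup reappears with query collision and the character's saved original walk speed is restored, so respawn and buff expiry share one timer.
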(event `self.Box.OnComponentBeginOverlap`
  (params (OverlappedComponent :type "PrimitiveComponent Object Reference") (OtherActor :type "Actor Object Reference") (OtherComp :type "PrimitiveComponent Object Reference") (OtherBodyIndex :type Integer) (bFromSweep :type Boolean) (SweepResult :type "HitResult Structure (by ref)"))
  (bind _asbp_player_character (cast `/Game/Blueprints/PlayerCharacter/BP_PlayerCharacter` OtherActor))
  (set `self.InstigatorCharacter` _asbp_player_character)
  (`self.Consume PowerUp`)
  (`KismetSystemLibrary.Delay` (`self.Duration`))
  (`self.Restore PowerUp`))

(event `Consume PowerUp`
  (`PrimitiveComponent.SetCollisionEnabled` (`self.Box`) "NoCollision")
  (`SceneComponent.SetVisibility` (`self.PowerUp`) false false)
  (`self.InstigatorCharacter`
    (:`then`
      (`self.Apply Buff`))
    (:`else`)))

(event `Restore PowerUp`
  (`PrimitiveComponent.SetCollisionEnabled` (`self.Box`) "QueryOnly")
  (`SceneComponent.SetVisibility` (`self.PowerUp`) true false)
  (`self.InstigatorCharacter`
    (:`then`
      (`self.Remove buff`))
    (:`else`)))

(event `Apply Buff`
  ;[1 1 1] Apply and Remove Buff
  (bind _instigatorcharacter (`self.InstigatorCharacter`)
    (:`then`
      (bind _charactermovement (`Character.CharacterMovement` _instigatorcharacter))
      (set `self.Original Walk Speed` (`CharacterMovementComponent.MaxWalkSpeed` _charactermovement))
      (set `CharacterMovementComponent.MaxWalkSpeed` (+ (`self.Original Walk Speed`) (`self.SpeedBuff`)) _charactermovement))
    (:`else`)))

(event `Remove buff`
  ;[1 1 1] Apply and Remove Buff
  (bind _instigatorcharacter (`self.InstigatorCharacter`)
    (:`then`
      (set `CharacterMovementComponent.MaxWalkSpeed` (`self.Original Walk Speed`) (`Character.CharacterMovement` _instigatorcharacter)))
    (:`else`)))

(fn `UserConstructionScript`)