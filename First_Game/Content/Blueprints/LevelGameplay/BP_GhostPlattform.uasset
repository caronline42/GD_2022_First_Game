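; BP_GhostPlattform is a level gameplay platform that stays hidden until a linked interruptor or sensor makes it appear.
; On BeginPlay it starts disappearing and binds to the interruptor's activate/deactivate events and the sensor's pawn enter/leave events, when those references are valid.
; Appear and Disappear play and reverse one timeline, which scales the Cube in X and Y with Z fixed at zero.
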(event `OnInterruptorActivated`
  ;[1 1 1] Interruptor Activation
  (`self.Appear`))

(event `OnInterruptorDesactivated`
  ;[1 1 1] Interruptor Activation
  (`self.Disappear`))

(event `self.ReceiveBeginPlay`
  (`self.Disappear`)
  (`|ExecutionSequence`
    (:`then_0`
      ;[1 1 1] Interruptor Activation
      (bind _interruptor (`self.Interruptor`)
        (:`then`
          (add `/Game/Blueprints/LevelGameplay/Interruptors/BP_Interruptor.OnInterruptorActivated` _interruptor (delegate `OnInterruptorActivated`))
          (add `/Game/Blueprints/LevelGameplay/Interruptors/BP_Interruptor.OnInterruptorDesactivated` _interruptor (delegate `OnInterruptorDesactivated`)))
        (:`else`)))
    (:`then_1`
      ;[1 1 1] Sensor Activation
      (bind _sensor (`self.Sensor`)
        (:`then`
          (add `/Game/Blueprints/LevelGameplay/BP_BasicCollider.OnPawnEnter` _sensor (delegate `Pawn Enter`))
          (add `/Game/Blueprints/LevelGameplay/BP_BasicCollider.OnPawnLeave` _sensor (delegate `Pawn Leave`)))
        (:`else`)))))

(event `Pawn Enter`
  ;[1 1 1] Sensor Activation
  (`self.Appear`))

(event `Pawn Leave`
  ;[1 1 1] Sensor Activation
  (`self.Disappear`))

(event `Appear`
  (bind (_direction _scaletrack) (`Timeline|Timeline_AppearDissapear` :!label _label)
    (:`Update`
      (bind _returnvalue (* 2 _scaletrack))
      (`SceneComponent.SetWorldScale3D` (`self.Cube`) (`KismetMathLibrary.MakeVector` _returnvalue _returnvalue)))))

(event `Disappear`
  (goto _label :!via `Reverse`))

(fn `UserConstructionScript`)