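; Health component that tracks its owner's hitpoints and destroys the owner when depleted.
; BeginPlay binds to the owner's any-damage event, which subtracts damage within zero and max, then broadcasts OnHealthChanged.
; The depletion check subtracts damage again from updated health before broadcasting OnHealthDepleted and destroying the owner.
; A Test event, also run at BeginPlay, prints health changes and death on screen.
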(event `Test`
  ;[1 1 1] Test
  (`/Engine/EditorBlueprintResources/StandardMacros.IsValid` (`self.GetOwner`)
    (:`Is Valid`
      (add `self.OnHealthChanged` (delegate `OnDamageTest`))
      (add `self.OnHealthDepleted` (delegate `OnDeath`)))))

(event `OnDamageTest`
  ;[1 1 1] Test
  (`KismetSystemLibrary.PrintString` (`KismetStringLibrary.Concat_StrStr` "Health: " (`KismetStringLibrary.Conv_DoubleToString` (`self.CrrentHitpoints`))) true true (struct :`R` 0.11238 :`G` 1.0 :`B` 0.468486 :`A` 1.0) 3.0))

(event `OnDeath`
  ;[1 1 1] Test
  (`KismetSystemLibrary.PrintString` "You Are Dead!" true true (struct :`R` 0.53 :`G` 0.015488 :`A` 1.0) 5.0))

(event `self.ReceiveBeginPlay`
  (bind _returnvalue (`self.GetOwner`))
  (`/Engine/EditorBlueprintResources/StandardMacros.IsValid` _returnvalue
    (:`Is Valid`
      (add `Actor.OnTakeAnyDamage` _returnvalue (delegate `OnDamageTaken`))
      (`self.Test`))))

(event `OnDamageTaken`
  (params (DamagedActor :type "Actor Object Reference") (Damage :type "Float (double-precision)") (DamageType :type "DamageType Object Reference") (InstigatedBy :type "Controller Object Reference") (DamageCauser :type "Actor Object Reference"))
  (bind _returnvalue (`self.GetOwner`))
  (bind _returnvalue_2 (`KismetMathLibrary.FClamp` (- (`self.CrrentHitpoints`) Damage) 0.0 (`self.MaxHitpoints`)))
  (set `self.CrrentHitpoints` _returnvalue_2)
  (`self.OnHealthChanged`)
  (if (<= _returnvalue_2 0.0)
    (`self.OnHealthDepleted`)
    (`/Engine/EditorBlueprintResources/StandardMacros.IsValid` _returnvalue
      (:`Is Valid`
        (`Actor.K2_DestroyActor` _returnvalue)))))